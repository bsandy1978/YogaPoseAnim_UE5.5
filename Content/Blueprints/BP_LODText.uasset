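; BP_LODText is a debug label actor that displays LOD sync information for a referenced MetaHuman actor.
; On Tick it checks that actor for a LODSyncComponent and writes the first one's debug text to its TextRender.
; Logic to scale the label by camera distance and field of view is present but never runs.
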(event `self.ReceiveTick`
  (params (DeltaSeconds :type "Float (single-precision)"))
  (bind _returnvalue (`self.K2_GetComponentsByClass` (`self.MetaHumanActor`) "/Script/Engine.LODSyncComponent"))
  ;[1 1 1] If we have a LODSyncComponent
  (if (> (`KismetArrayLibrary.Array_Length` _returnvalue) 0)
    ;[1 1 1] Set text to show debug info
    (`TextRenderComponent.K2_SetText` (`self.TextRender`) (`KismetTextLibrary.Conv_StringToText` (`LODSyncComponent.GetLODSyncDebugText` (`|GetArrayItem` _returnvalue))))))

(fn `UserConstructionScript`)